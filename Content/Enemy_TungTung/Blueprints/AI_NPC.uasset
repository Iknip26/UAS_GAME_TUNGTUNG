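; AI controller for the TungTung enemy, driving it with a blackboard and behavior tree.
; On BeginPlay it resets blackboard keys, sets the level manager's used path to the downstairs path list, then runs the tree.
; Sight perception of the player updates the target key and raises the pawn's walk speed.
; Losing sight stores the last seen location and lowers the speed.
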(event OnTargetPerceptionUpdated(AIPerception)
  (params (Actor :type Actor%20Object%20Reference) (Stimulus :type AI%20Stimulus%20Structure))
  (CallFunction|HandleSightSense Actor Stimulus))

(event EventBeginPlay
  (bind _blackboardcomponent (Class|AIController|UseBlackboard "/Game/Enemy_TungTung/Blueprints/AI/BT/BB_NPC_2.BB_NPC_2"))
  (Variables|Default|SetblackboardRef _blackboardcomponent)
  (bind _returnvalue (Actor|GetActorOfClass "/Game/Blueprints/BP_LevelManager.BP_LevelManager_C"))
  (Variables|Default|SetLvlManagerRef _returnvalue)
  (CallFunction|ResetAtribute)
  (Variables|/Game/Blueprints/BP_LevelManager.BP_LevelManager_C|SetusedPath _returnvalue (Variables|/Game/Blueprints/BP_LevelManager.BP_LevelManager_C|GetDownPathList _returnvalue))
  (AI|RunBehaviorTree "/Game/Enemy_TungTung/Blueprints/AI/BT/BT_NPC_2.BT_NPC_2"))

(event EventTick
  (params (DeltaSeconds :type Float%20%28single-precision%29)))

(fn ConstructionScript)

(fn HandleSightSense
  (params (Actor :type Actor%20Object%20Reference%20%28by%20ref%29) (Stimulus :type AI%20Stimulus%20Structure%20%28by%20ref%29))
  (bind _returnvalue (Class|AIPerceptionSystem|GetSenseClassforStimulus Stimulus))
  (if (== _returnvalue "/Script/AIModule.AISense_Sight")
    (if (== Actor (Game|GetPlayerCharacter 0))
      (AI|Components|Blackboard|SetValueasObject (Variables|Default|GetBlackboard) (Utilities|Name|MakeLiteralName "targetActor") (Utilities|SelectObject (Game|GetPlayerCharacter 0) 0 (.bsuccessfullysensed Stimulus)))
      (bind _asbp_tung_tung (Utilities|Casting|CastToBP_TungTung (Pawn|GetControlledPawn)))
      (if (.bsuccessfullysensed Stimulus)
        (Variables|/Script/Engine.CharacterMovementComponent|SetMaxWalkSpeed (Variables|/Script/Engine.Character|GetCharacterMovement _asbp_tung_tung) 4e+02)
        (else
          (AI|Components|Blackboard|SetValueasVector (Variables|Default|GetBlackboard) (Utilities|Name|MakeLiteralName "lastLocation") (.stimuluslocation Stimulus))
          (Variables|/Script/Engine.CharacterMovementComponent|SetMaxWalkSpeed (Variables|/Script/Engine.Character|GetCharacterMovement _asbp_tung_tung) 2.5e+02)))
      (else
        (return)))
    (else
      (return))))

(fn ResetAtribute
  (bind _blackboardcomponent (Class|AIController|UseBlackboard "/Game/Enemy_TungTung/Blueprints/AI/BT/BB_NPC_2.BB_NPC_2"))
  (AI|Components|Blackboard|ClearValue _blackboardcomponent (Utilities|Name|MakeLiteralName "targetActor"))
  (AI|Components|Blackboard|ClearValue _blackboardcomponent (Utilities|Name|MakeLiteralName "targetActor"))
  (AI|Components|Blackboard|SetValueasBool _blackboardcomponent (Utilities|Name|MakeLiteralName "isInUpFloor") false)
  (AI|Components|Blackboard|SetValueasBool _blackboardcomponent (Utilities|Name|MakeLiteralName "isWalking") false))