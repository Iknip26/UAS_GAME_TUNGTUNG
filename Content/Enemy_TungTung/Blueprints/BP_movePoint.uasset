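; BP_movePoint is a waypoint actor for the TungTung enemy that caches a list of its nearest neighboring move points.
; On BeginPlay it gathers every other BP_movePoint in the level and records each one's distance from itself.
; A hand-written selection sort orders them nearest first, then the result is stored in ClosePointList and resized to ClosePointLimit.
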(event EventBeginPlay
  (bind _outputarray (CallFunction|GetClosestPoints))
  (bind _outputarray_2 (CallFunction|SortDistance _outputarray))
  (bind _output_get (Variables|Default|SetclosePointList _outputarray_2))
  (Utilities|Array|Resize _output_get (Variables|Default|GetclosePointLimit)))

(event Collision|EventActorBeginOverlap
  (params (OtherActor :type Actor%20Object%20Reference)))

(event EventTick
  (params (DeltaSeconds :type Float%20%28single-precision%29)))

(fn ConstructionScript)

(fn GetClosestPoints
  (bind _self self)
  (bind _outactors (Actor|GetAllActorsOfClass "BP_movePoint_C"))
  (for _array_element _outactors
    (if (!= _array_element _self)
      (bind _newparam (CallFunction|CountDistance _array_element _self))
      (Utilities|Array|Add (LocalVariables|GetclosestPointList) (Utilities|Struct|MakeclosestPointData _array_element _newparam))))
  (return (LocalVariables|GetclosestPointList)))

(fn CountDistance
  (params (point :type BP%20Move%20Point%20Object%20Reference) (origin :type BP%20Move%20Point%20Object%20Reference))
  (return (Math|Vector|Distance(Vector) (Transformation|GetActorLocation point) (Transformation|GetActorLocation origin))))

(fn SortDistance
  (params (inputArray :type Array%20of%20Closest%20Point%20Data%20Structures))
  (for (_ _array_index) inputArray
    (bind _output_get (LocalVariables|Setmin _array_index))
    (for _index (range (+ _array_index 1) (- (Utilities|Array|Length inputArray) 1))
      (if (< (.distance (Utilities|Array|Get(acopy) inputArray _index)) (.distance (Utilities|Array|Get(acopy) inputArray _output_get)))
        (bind _output_get_2 (LocalVariables|Setmin _index))))
    (if (!= _array_index (LocalVariables|Getmin))
      (Utilities|Array|Swap inputArray _output_get_2 _array_index)))
  (return inputArray))