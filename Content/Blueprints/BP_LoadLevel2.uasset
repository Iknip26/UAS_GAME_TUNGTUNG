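; Interactable level-transition actor that loads ThirdPersonMap when E is pressed while an actor overlaps it.
; BeginPlay enables input from player controller 0, and begin/end overlap events toggle an IsOverlapping flag without checking which actor overlaps.
; On E, it clears all widgets, shows a LoadingScreen widget, waits briefly, opens the level, then hides the cursor and sets game-only input.
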(event EventBeginPlay
  (Input|EnableInput (Game|GetPlayerController 0)))

(event Collision|EventActorBeginOverlap
  (params (OtherActor :type Actor%20Object%20Reference))
  (Variables|Default|SetbIsOverlapping true))

(event Collision|EventActorEndOverlap
  (params (OtherActor :type Actor%20Object%20Reference))
  (Variables|Default|SetbIsOverlapping false))

(event Input|KeyboardEvents|E
  (params (Key :type Key%20Structure :default "None"))
  (bind _returnvalue (Game|GetPlayerController 0))
  (:Pressed
    (if (Variables|Default|GetbIsOverlapping)
      (Viewport|RemoveAllWidgets)
      (bind _returnvalue_2 (UserInterface|CreateWidget "/Game/UI/LoadingScreen.LoadingScreen_C" _returnvalue))
      (UserInterface|Viewport|AddtoViewport _returnvalue_2 0)
      (Utilities|FlowControl|Delay 0.5)
      (Game|OpenLevel(byName) "ThirdPersonMap")
      (Variables|/Script/Engine.PlayerController|SetbShowMouseCursor _returnvalue false)
      (Input|SetInputModeGameOnly _returnvalue false))))

(fn ConstructionScript)