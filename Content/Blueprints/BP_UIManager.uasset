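; BP_UIManager is a UI manager Blueprint that toggles a pause menu widget.
; BeginPlay creates a UI_Pause widget but sets UIPause to None rather than to the created widget.
; PauseGame adds UIPause to the viewport or removes it based on the IsGamePaused flag, then flips that flag.
; It only changes the widget and flag, without calling the engine's pause.
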(event EventBeginPlay
  (UserInterface|CreateWidget "/Game/ThirdPerson/Blueprints/UI_Pause.UI_Pause_C")
  (Variables|Default|SetUI_Pause 0))

(event Collision|EventActorBeginOverlap
  (params (OtherActor :type Actor%20Object%20Reference)))

(event EventTick
  (params (DeltaSeconds :type Float%20%28single-precision%29)))

(fn ConstructionScript)

(fn PauseGame
  (bind _ui_pause (Variables|Default|GetUI_Pause))
  (if (Variables|Default|GetisGamePaused?)
    (Widget|RemovefromParent _ui_pause)
    (else
      (UserInterface|Viewport|AddtoViewport _ui_pause 0)))
  (if (Variables|Default|GetisGamePaused?)
    (Variables|Default|SetisGamePaused? false)
    (else
      (Variables|Default|SetisGamePaused? true))))