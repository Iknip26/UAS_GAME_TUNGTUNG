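; BP_LevelManager is a level manager that handles the player's lives and the initial state of the level's doors.
; On BeginPlay, CloseAllDoor calls Interact on every BP_Door, relying on that call to close them.
; The Die event loads MainMenuMap as game over on the last life.
; Otherwise, it decrements Live and moves the existing first-person character to a PlayerStart, without respawning the actor or resetting the level.
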(event Custom|Die
  (if (== (Variables|Default|GetLive) 1)
    ;[1 1 1] Game Over
    (Game|OpenLevel(byName) "MainMenuMap")
    (Development|PrintString "Game Over")
    (else
      ;[1 1 1] Respawn
      (Variables|Default|SetLive (- (Variables|Default|GetLive) 1))
      (bind _returnvalue (Actor|GetActorOfClass "/Game/FirstPerson/Blueprints/BP_FirstPersonCharacter.BP_FirstPersonCharacter_C"))
      (bind _returnvalue_2 (Actor|GetActorOfClass "/Script/Engine.PlayerStart"))
      (Transformation|SetActorLocation _returnvalue (Transformation|GetActorLocation _returnvalue_2) false false)
      (Development|PrintString (Utilities|String|ToString(Integer) (Variables|Default|GetLive))))))

(event EventBeginPlay
  (CallFunction|CloseAllDoor))

(event Collision|EventActorBeginOverlap
  (params (OtherActor :type Actor%20Object%20Reference)))

(event EventTick
  (params (DeltaSeconds :type Float%20%28single-precision%29)))

(fn ConstructionScript)

(fn CloseAllDoor
  (bind _outactors (Actor|GetAllActorsOfClass "/Game/Blueprints/BP_Door.BP_Door_C"))
  (for _array_element _outactors
    (Default|Interact _array_element)))