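; BP_Doo is a door actor that toggles open and closed and opens automatically for BP_TungTung enemies.
; DoorCollider overlaps flag when a BP_TungTung is inside, and Tick calls Interact while the flag is set and the door is closed.
; Interact flips IsOpen, snaps the mesh's relative rotation to actor rotation plus an open or close yaw offset, and prints the state.
; Leaving the collider does not close the door.
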(event OnComponentBeginOverlap(DoorCollider)
  (params (OverlappedComponent :type Primitive%20Component%20Object%20Reference) (OtherActor :type Actor%20Object%20Reference) (OtherComp :type Primitive%20Component%20Object%20Reference) (OtherBodyIndex :type Integer) (bFromSweep :type Boolean) (SweepResult :type Hit%20Result%20Structure%20%28by%20ref%29))
  (Utilities|Casting|CastToBP_TungTung OtherActor)
  (Variables|Default|SetisEnemyInside? true))

(event OnComponentEndOverlap(DoorCollider)
  (params (OverlappedComponent :type Primitive%20Component%20Object%20Reference) (OtherActor :type Actor%20Object%20Reference) (OtherComp :type Primitive%20Component%20Object%20Reference) (OtherBodyIndex :type Integer))
  (Utilities|Casting|CastToBP_TungTung OtherActor)
  (Variables|Default|SetisEnemyInside? false))

(event EventBeginPlay)

(event Collision|EventActorBeginOverlap
  (params (OtherActor :type Actor%20Object%20Reference)))

(event EventTick
  (params (DeltaSeconds :type Float%20%28single-precision%29))
  (if (Variables|Default|GetisEnemyInside?)
    (if (not (Variables|Default|GetisOpen?))
      (CallFunction|Interact))))

(fn ConstructionScript)

(fn Interact
  (bind _returnvalue (Transformation|GetActorRotation))
  (if (Variables|Default|GetisOpen?)
    (LocalVariables|SetRotatorValue (Variables|Default|GetcloseRotation))
    (Variables|Default|SetisOpen? false)
    (else
      (LocalVariables|SetRotatorValue (Variables|Default|GetopenRotation))
      (Variables|Default|SetisOpen? true)))
  (Transformation|SetRelativeRotation (Variables|Default|Getmesh) (Math|Rotator|MakeRotator (.roll _returnvalue) (.pitch _returnvalue) (+ (.yaw _returnvalue) (LocalVariables|GetRotatorValue))) false false)
  (Development|PrintString (Utilities|String|ToString(Boolean) (Variables|Default|GetisOpen?)))
  (return 0))