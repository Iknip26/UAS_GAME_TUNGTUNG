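; BP_Item is a pickup item actor that the first-person character can grab by interacting with it.
; Interact does its work only when the item is not placed, passing the item's static mesh and a self reference to BP_FirstPersonCharacter's SetGrabbedItem.
; It then triggers DestroyItem, which removes the actor after a short delay, and plays a 2D pickup sound.
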(event Custom|Destroy%20Item
  (Utilities|FlowControl|Delay 0.2)
  (Actor|DestroyActor))

(fn ConstructionScript)

(fn Interact
  (if (not (Variables|Default|GetisItemPlaced))
    (bind _returnvalue (Actor|GetActorOfClass "/Game/FirstPerson/Blueprints/BP_FirstPersonCharacter.BP_FirstPersonCharacter_C"))
    (Default|SetGrabbedItem _returnvalue (Variables|/Script/Engine.StaticMeshComponent|GetStaticMesh (Variables|Default|GetItemMesh)) self)
    (CallFunction|DestroyItem)
    (Audio|SpawnSound2D "/Game/SFX/pickup_sfx_Cue.pickup_sfx_Cue" 2.0 1.0 0.0 0)
    (return 0)))